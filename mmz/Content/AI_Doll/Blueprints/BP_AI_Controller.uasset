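; AI controller for a doll enemy that freezes while on screen and advances on the player when unseen.
; It runs BT_AI_Doll and feeds its blackboard a target from sight perception, an optional immediate chase, or an optional first-look activation.
; Tick polls WasRecentlyRendered on the doll's RenderPoint to toggle CanMove, easing speed to zero when seen and restoring it when unseen.
; While unseen, a sphere trace damages nearby pawns.
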(event `Clear Target`
  ;[0 0 0] Clear Target
  (`BlackboardComponent.SetValueAsObject` (`AIBlueprintHelperLibrary.GetBlackboard` null) "TargetActor" null)
  (`self.SetActorTickEnabled` false)
  (`self.StopMovement`)
  (set `self.CanAttack` false)
  (`BlackboardComponent.SetValueAsBool` (`AIBlueprintHelperLibrary.GetBlackboard` null) "CanMove" false))

(event `self.ReceiveBeginPlay`
  ;[0 0 0] Begin Play - Run Behavior Tree
  (`self.RunBehaviorTree` "/Game/AI_Doll/Artificial_Intelligence/BT_AI_Doll.BT_AI_Doll")
  (set `CharacterMovementComponent.MaxWalkSpeed` 0.0 (`Character.CharacterMovement` (`self.As BP AI Doll`))))

(event `self.AIPerception.OnTargetPerceptionUpdated`
  (params (Actor :type "Actor Object Reference") (Stimulus :type "AIStimulus Structure"))
  ;[0 0 0] Perception Updated
  (`self.Sight` Stimulus Actor))

(event `self.ReceivePossess`
  (params (PossessedPawn :type "Pawn Object Reference"))
  (bind _returnvalue (`GameplayStatics.GetPlayerCharacter` 0))
  ;[0 0 0] Set Pawn Ref
  (set `self.Possessed Pawn` PossessedPawn)
  (bind _asbp_ai_doll (cast `/Game/AI_Doll/Blueprints/BP_AI_Doll` (`self.Possessed Pawn`)))
  (set `self.As BP AI Doll` _asbp_ai_doll)
  ;[0 0 0] Start Chasing the player right away?
  (if (`self.Start Chasing the Player Right Away`)
    (`/Engine/EditorBlueprintResources/StandardMacros.IsValid` (`AIBlueprintHelperLibrary.GetBlackboard` null) :!label _label
      (:`Is Valid`
        (`/Engine/EditorBlueprintResources/StandardMacros.IsValid` _returnvalue :!label _label_2
          (:`Is Valid`
            (`BlackboardComponent.SetValueAsObject` (`AIBlueprintHelperLibrary.GetBlackboard` null) "TargetActor" _returnvalue)
            (`self.SetActorTickEnabled` true))
          (:`Is Not Valid`
            (`KismetSystemLibrary.Delay` 0.5)
            (goto _label_2))))
      (:`Is Not Valid`
        (`KismetSystemLibrary.Delay` 0.5)
        (goto _label)))))

(event `self.ReceiveTick`
  (params (DeltaSeconds :type "Float (single-precision)"))
  ;[0 0 0] Event Tick
  (if (`self.Player sees the AI`)
    ;;[0 0 0] Additional ///// The AI ​​will be activated if the Player looks at the AI ​​first
    (if (`self.Rendered`)
      (`self.AI Activated` :!label _label_3
        (:`True`
          (`|ExecutionSequence`
            (:`then_0`
              (if (`self.CanAttack`)
                (if (`BlackboardComponent.GetValueAsBool` (`AIBlueprintHelperLibrary.GetBlackboard` null) "CanMove")
                  (if (`BlackboardComponent.GetValueAsBool` (`AIBlueprintHelperLibrary.GetBlackboard` null) "CanMove") :!label _label_4
                    (`/Engine/EditorBlueprintResources/StandardMacros.DoOnce` false :!label _label_5
                      (:`Completed`
                        (set `CharacterMovementComponent.MaxWalkSpeed` (`/Game/AI_Doll/Blueprints/BP_AI_Doll.MaxWalkSpeed` (`self.As BP AI Doll`)) (`Character.CharacterMovement` (`self.As BP AI Doll`))))))
                  (else
                    (bind _output_get (set `CharacterMovementComponent.MaxWalkSpeed` (`KismetMathLibrary.FInterpTo` (`CharacterMovementComponent.MaxWalkSpeed` (`Character.CharacterMovement` (`self.As BP AI Doll`))) 0.0 (`GameplayStatics.GetWorldDeltaSeconds`) 3.0) (`Character.CharacterMovement` (`self.As BP AI Doll`))))
                    (if (`KismetMathLibrary.NearlyEqual_FloatFloat` _output_get 0.0 1.0)
                      (`|ExecutionSequence`
                        (:`then_0`
                          (`MovementComponent.StopMovementImmediately` (`Character.CharacterMovement` (`self.As BP AI Doll`)))
                          (set `self.CanAttack` false))
                        (:`then_1`
                          (goto _label_6 :!via `Reset`)))
                      (else
                        (`/Engine/EditorBlueprintResources/StandardMacros.DoOnce` false :!label _label_6
                          (:`Completed`
                            ;;[0 0 0] Target Location
                            (`BlackboardComponent.SetValueAsVector` (`AIBlueprintHelperLibrary.GetBlackboard` null) "TargetLocation" (`self.K2_GetActorLocation` (`self.Target Actor`)))))))))
                (else
                  (goto _label_4))))
            (:`then_1`
              ;;[0 0 0] Is Rendered
              (if (`PrimitiveComponent.WasRecentlyRendered` (`/Game/AI_Doll/Blueprints/BP_AI_Doll.RenderPoint` (`self.As BP AI Doll`)) 0.2)
                (`|ExecutionSequence`
                  (:`then_0`
                    (`/Engine/EditorBlueprintResources/StandardMacros.DoOnce` false :!label _label_7
                      (:`Completed`
                        (`KismetSystemLibrary.Delay` 0.1)
                        (goto _label_8 :!via `Open`))))
                  (:`then_1`
                    (`/Engine/EditorBlueprintResources/StandardMacros.Gate` true :!label _label_8
                      (:`Exit`
                        ;;[0 0 0] Frozen
                        (`BlackboardComponent.SetValueAsBool` (`AIBlueprintHelperLibrary.GetBlackboard` null) "CanMove" false)
                        (set `self.CanAttack` true))))
                  (:`then_2`
                    (`self.Reset - Max Speed`)))
                (else
                  (`BlackboardComponent.SetValueAsBool` (`AIBlueprintHelperLibrary.GetBlackboard` null) "CanMove" true)
                  (`self.Object Trace`)
                  (`|ExecutionSequence`
                    (:`then_0`
                      (goto _label_7 :!via `Reset`))
                    (:`then_1`
                      (goto _label_8 :!via `Close`)))))))))
      (else
        ;;;[0 0 0] Is Rendered
        (if (`PrimitiveComponent.WasRecentlyRendered` (`/Game/AI_Doll/Blueprints/BP_AI_Doll.RenderPoint` (`self.As BP AI Doll`)) 0.2)
          (set `self.Rendered` true)
          (`BlackboardComponent.SetValueAsObject` (`AIBlueprintHelperLibrary.GetBlackboard` null) "TargetActor" (`GameplayStatics.GetPlayerCharacter` 0)))))
    (else
      (goto _label_3))))

(event `Reset - Max Speed`
  ;[0 0 0] Event Tick
  (goto _label_5 :!via `Reset`))

(fn `Check if the player sees the AI`
  (params (Condition :type Boolean))
  ;[0 0 0] Check if the player sees the artificial intelligence
  (if Condition
    (`BlackboardComponent.SetValueAsBool` (`AIBlueprintHelperLibrary.GetBlackboard` null) "CanMove" false)
    (bind _output_get (set `CharacterMovementComponent.MaxWalkSpeed` (`KismetMathLibrary.FInterpTo` (`CharacterMovementComponent.MaxWalkSpeed` (`Character.CharacterMovement` (`self.As BP AI Doll`))) 0.0 (`GameplayStatics.GetWorldDeltaSeconds`) 1.0) (`Character.CharacterMovement` (`self.As BP AI Doll`))))
    (if (`KismetMathLibrary.NearlyEqual_FloatFloat` _output_get 0.0 1.0)
      (`MovementComponent.StopMovementImmediately` (`Character.CharacterMovement` (`self.As BP AI Doll`))))))

(fn `Object Trace`
  (bind _returnvalue (`self.K2_GetActorLocation` (`self.Possessed Pawn`)))
  ;[0 0 0] Object Trace - Damage
  (bind (_outhit _returnvalue_2) (`KismetSystemLibrary.SphereTraceSingleForObjects` _returnvalue _returnvalue 100.0 (`|MakeArray` "ObjectTypeQuery3" :!type "EObjectTypeQuery Enum") false (`|MakeArray` self :!type "Actor Object Reference")))
  (if _returnvalue_2
    (`GameplayStatics.ApplyDamage` (`.HitActor` (`GameplayStatics.BreakHitResult` _outhit)) 5.0 null (`self.Possessed Pawn`))))

(fn `Sight`
  (params (Stimulus :type "AIStimulus Structure (by ref)") (Actor :type "Actor Object Reference"))
  ;[0 0 0] Sight
  (bind _returnvalue (`AIPerceptionSystem.GetSenseClassForStimulus` Stimulus))
  (if (== _returnvalue "/Script/AIModule.AISense_Sight")
    (if (`.bSuccessfullySensed` (break `AIStimulus` (`local.Stimulus`)))
      (if (== (`local.Actor`) (`GameplayStatics.GetPlayerCharacter` 0))
        (`self.Target Actor`
          (:`then`
            _)
          (:`else`
            (set `self.Target Actor` (`local.Actor`))))
        (`BlackboardComponent.SetValueAsObject` (`AIBlueprintHelperLibrary.GetBlackboard` null) "TargetActor" (`self.Target Actor`))
        (`self.SetActorTickEnabled` true)))))

(fn `UserConstructionScript`)