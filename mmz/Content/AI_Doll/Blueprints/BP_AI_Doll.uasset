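; AI doll actor that gives its three sphere meshes a shared dynamic eye material and contains logic for a creepy voice line.
; The voice logic turns the eyes red and uses a looping timer to ease pitch toward normal when blackboard CanMove is true, otherwise toward zero.
; Audio completion clears the timer and turns the eyes white.
; PlayVoice is empty, and the chain that starts the voice is unconnected.
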(event `self.ReceiveBeginPlay`
  ;[0 0 0] Begin Play - Create Dynamic Material
  (bind _returnvalue (`KismetMaterialLibrary.CreateDynamicMaterialInstance` "/Game/AI_Doll/Demo/Characters/Mannequins/Materials/M_Eye.M_Eye"))
  (bind _output_get (set `self.Dynamic Material` _returnvalue))
  (`PrimitiveComponent.SetMaterial` (`self.Sphere2`) 0 _output_get)
  (`PrimitiveComponent.SetMaterial` (`self.Sphere1`) 0 _output_get)
  (`PrimitiveComponent.SetMaterial` (`self.Sphere`) 0 _output_get))

(event `Play Voice`
  ;[0 0 0] Voice
)

(event `CustomEvent_1`
  ;[0 0 0] Voice
  (`KismetSystemLibrary.K2_ClearAndInvalidateTimerHandle` (`self.Timer`))
  (`MaterialInstanceDynamic.SetVectorParameterValue` (`self.Dynamic Material`) "Color" (struct :`R` 1.0 :`G` 1.0 :`B` 1.0 :`A` 1.0))
  (set `self.Current Audio` null))

(event `CustomEvent_0`
  ;[0 0 0] Voice
  (if (`BlackboardComponent.GetValueAsBool` (`AIBlueprintHelperLibrary.GetBlackboard` (`self.GetController`)) "CanMove")
    (bind _current_audio (`self.Current Audio`)
      (:`then`
        (`AudioComponent.SetPitchMultiplier` _current_audio (`KismetMathLibrary.FInterpTo` (`AudioComponent.PitchMultiplier` (`self.Current Audio`)) 1.0 (`GameplayStatics.GetWorldDeltaSeconds`) 1.0)))
      (:`else`))
    (else
      (bind _current_audio_2 (`self.Current Audio`)
        (:`then`
          (`AudioComponent.SetPitchMultiplier` _current_audio_2 (`KismetMathLibrary.FInterpTo_Constant` (`AudioComponent.PitchMultiplier` (`self.Current Audio`)) 0.0 (`GameplayStatics.GetWorldDeltaSeconds`) 0.2)))
        (:`else`)))))

(fn `UserConstructionScript`)