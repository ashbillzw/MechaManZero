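; BP_Enemy is a damageable enemy actor with a text label above it showing its current HP.
; TakeDamage subtracts clamped damage, then starts a timer-based immunity window that blocks further hits until it resets.
; UpdateHP refreshes the label and destroys the actor when HP reaches zero.
; Each Tick, the text rotates to face the player camera.
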(event `UpdateHP`
  (`TextRenderComponent.K2_SetText` (`self.TextRender`) (`KismetTextLibrary.Conv_StringToText` (`KismetStringLibrary.Conv_DoubleToString` (`self.HP`))))
  (if (<= (`self.HP`) 0.0)
    (`self.K2_DestroyActor`)))

(event `self.ReceiveBeginPlay`
  (`self.UpdateHP`))

(event `ResetBCanTakeDamage`
  (set `self.bCanTakeDamage` true))

(event `/Game/Characters/Enemy/BPI_Damageable.TakeDamage`
  (params (Float :type "Float (double-precision)") (`Hit Result` :type "HitResult Structure") (Causer :type "Actor Object Reference"))
  (if (and (`self.bIsAlive`) (`self.bCanTakeDamage`))
    (set `self.bCanTakeDamage` false)
    (`KismetSystemLibrary.K2_SetTimerDelegate` (delegate `ResetBCanTakeDamage`) (`self.ImmuneTime`))
    (bind _output_get (set `self.HP` (`KismetMathLibrary.FClamp` (- (`self.HP`) Float) 0.0 (`self.MaxHP`))))
    (`self.UpdateHP`)
    (if (<= _output_get 0.0)
      (set `self.bIsAlive` false))))

(event `self.ReceiveTick`
  (params (DeltaSeconds :type "Float (single-precision)"))
  (bind _textrender (`self.TextRender`))
  (`SceneComponent.K2_SetWorldRotation` _textrender (`KismetMathLibrary.FindLookAtRotation` (`SceneComponent.K2_GetComponentLocation` _textrender) (`PlayerCameraManager.GetCameraLocation` (`PlayerController.PlayerCameraManager` (`GameplayStatics.GetPlayerController` 0)))) false false))

(fn `UserConstructionScript`)